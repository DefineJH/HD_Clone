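; Enemy AI controller that sets and clears the Blackboard TargetActor from perception updates.
; With no valid target, it stores any updated actor tagged Player, without checking whether it was sensed or lost.
; With a valid target, it clears the key only if the controller itself has the Player tag.
; Both branches print debug strings, and a debug sphere draw is left unconnected.
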(event OnPerceptionUpdated(PerceptionComponent)
  (params (UpdatedActors :type Array%20of%20Actor%20Object%20References))
  (Utilities|IsValid (AI|Components|Blackboard|GetValueasObject (AI|GetBlackboard 0) (Utilities|Name|MakeLiteralName "TargetActor"))
    (:Is%20Valid
      (if (Actor|ActorHasTag "Player")
        (AI|Components|Blackboard|SetValueasObject (AI|GetBlackboard 0) (Utilities|Name|MakeLiteralName "TargetActor") 0)
        (Development|PrintString "나")))
    (:Is%20Not%20Valid
      (for _array_element UpdatedActors
        (if (Actor|ActorHasTag _array_element "Player")
          (AI|Components|Blackboard|SetValueasObject (AI|GetBlackboard 0) (Utilities|Name|MakeLiteralName "TargetActor") _array_element)
          (Development|PrintString "들"))))))

(event EventTick
  (params (DeltaSeconds :type Float%20%28single-precision%29)))

(fn ConstructionScript)